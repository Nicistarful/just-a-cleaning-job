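; InstancedModularPiece is a modular building piece that tiles one static mesh into a flat Length by Width grid.
; The construction script adds the copies to an InstancedStaticMesh component, with Width columns along X and rows along Y.
; Spacing is twice the mesh's bounding-box maximum on each axis, so tiles abut when the pivot is centered.
; The event graph holds only disabled placeholder events.
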(fn `UserConstructionScript`
  (bind _width (`self.Width`))
  (for _index (range (* (`self.Length`) (`self.Width`)))
    (`InstancedStaticMeshComponent.AddInstance` (`self.InstancedStaticMesh`) (`KismetMathLibrary.MakeTransform` (`KismetMathLibrary.MakeVector` (* (mod _index _width) (* (.x (`.Max` (break `Box` (`StaticMesh.GetBoundingBox` (`StaticMeshComponent.StaticMesh` (`self.InstancedStaticMesh`)))))) 2.0)) (* (/ _index _width) (* (.y (`.Max` (break `Box` (`StaticMesh.GetBoundingBox` (`StaticMeshComponent.StaticMesh` (`self.InstancedStaticMesh`)))))) 2.0)))))))