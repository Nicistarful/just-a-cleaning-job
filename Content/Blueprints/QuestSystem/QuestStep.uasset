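; QuestStep is one stage of a quest, holding a list of quest targets and a task description.
; On BeginPlay it registers itself with each target, and ActivateTargets marks them all active.
; RemoveTarget drops a target from the list; once the list is empty, the step removes itself from its Quest and prints the task in red.
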(event `self.ReceiveBeginPlay`
  (for _array_element (`self.QuestTargets`)
    (set `/Game/Blueprints/QuestSystem/QuestTarget.QuestStep` self _array_element)))

(event `ActivateTargets`
  (for _array_element (`self.QuestTargets`)
    (set `/Game/Blueprints/QuestSystem/QuestTarget.Active` true _array_element)))

(event `RemoveTarget`
  (params (QuestTarget :type "/Game/Blueprints/QuestSystem/QuestTarget Object Reference"))
  (`KismetArrayLibrary.Array_RemoveItem` (`self.QuestTargets`) QuestTarget)
  (if (`self.IsCompleted`)
    (`/Game/Blueprints/QuestSystem/Quest.RemoveStep` (`self.Quest`) self)
    (`KismetSystemLibrary.PrintString` (`KismetTextLibrary.Conv_TextToString` (`self.Task`)) true true (struct :`R` 1.0 :`B` 0.006044 :`A` 1.0))))

(fn `IsCompleted`
  (returns (ReturnValue :type Boolean))
  (return (== (`KismetArrayLibrary.Array_Length` (`self.QuestTargets`)) 0)))

(fn `UserConstructionScript`)