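; Quest actor that holds an objective, a list of step actors and rewards, and manages its lifecycle from start to completion.
; On BeginPlay it links each step to itself, and StartQuest activates every step's targets at once and notifies the QuestManager.
; RemoveStep destroys a step and reports it to the manager.
; When no steps remain, it activates reward messages, signals completion and destroys itself.
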(event `self.ReceiveBeginPlay`
  (for _array_element (`self.QuestSteps`)
    (set `/Game/Blueprints/QuestSystem/QuestStep.Quest` self _array_element)))

(event `StartQuest`
  (for _array_element (`self.QuestSteps`)
    (`KismetSystemLibrary.PrintString` (`KismetTextLibrary.Conv_TextToString` (`/Game/Blueprints/QuestSystem/QuestStep.Task` _array_element)) true true (struct :`G` 1.0 :`B` 0.016063 :`A` 1.0))
    (`/Game/Blueprints/QuestSystem/QuestStep.ActivateTargets` _array_element))
  (`KismetSystemLibrary.PrintString` (`KismetTextLibrary.Conv_TextToString` (`self.Objective`)) true true (struct :`R` 0.000854 :`G` 1.0 :`A` 1.0))
  (`/Game/Blueprints/QuestSystem/QuestManager.OnQuestStarted` (`self.QuestManager`) self))

(event `RemoveStep`
  (params (QuestStep :type "/Game/Blueprints/QuestSystem/QuestStep Object Reference"))
  (`KismetArrayLibrary.Array_RemoveItem` (`self.QuestSteps`) QuestStep)
  (`self.K2_DestroyActor` QuestStep)
  (`/Game/Blueprints/QuestSystem/QuestManager.OnQuestStepCompleted` (`self.QuestManager`))
  (if (`self.IsCompleted`)
    (`self.FinishQuest`)))

(event `FinishQuest`
  (for _array_element (`self.Reward`)
    (message `/Game/Blueprints/QuestSystem/QuestingInterface.ActivateReward` _array_element))
  (`KismetSystemLibrary.PrintString` (`KismetTextLibrary.Conv_TextToString` (`self.Objective`)) true true (struct :`R` 1.0 :`B` 0.062383 :`A` 1.0))
  (`/Game/Blueprints/QuestSystem/QuestManager.OnQuestCompleted` (`self.QuestManager`))
  (`self.K2_DestroyActor`))

(fn `IsCompleted`
  (returns (ReturnValue :type Boolean))
  (return (== (`KismetArrayLibrary.Array_Length` (`self.QuestSteps`)) 0)))

(fn `UserConstructionScript`)