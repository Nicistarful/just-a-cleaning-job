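; BP_Door is an interactable, lockable door that teleports the player to its other side behind a screen fade.
; Front and Back overlaps track the player's side, and a map built in the construction script pairs each with the opposite teleport point.
; Interacting while locked tries a BP_Key item or plays a locked sound with an optional notification.
; When unlocked, it disables input, fades out, teleports, fades in and restores input.
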(event `/Game/Blueprints/Interfaces/Interaction.Interact`
  (params (InteractionItem :type "Actor Object Reference"))
  (bind _value (`BlueprintMapLibrary.Map_Find` (`self.TeleportMapping`) (`self.CurrentCollider`)))
  (if (`self.IsLocked`)
    (bind _asbp_key (cast `/Game/Blueprints/Door/BP_Key` InteractionItem)
      (:`then`
        (`self.Unlock` _asbp_key))
      (:`CastFailed`
        (`GameplayStatics.PlaySoundAtLocation` "/Game/Sound/Door/door-locked.door-locked" (`self.K2_GetActorLocation`) (struct) 1.0 1.0 0.0 null null null)
        (if (`self.ShowPrompt`)
          (`/Game/Blueprints/UI/NotificationComponent.NotifyPlayer` (`self.NotificationComponent`)))))
    (else
      (`/Engine/EditorBlueprintResources/StandardMacros.IsValid` (`self.CurrentCollider`)
        (:`Is Valid`
          (`self.DisableInput` (`GameplayStatics.GetPlayerCharacter` 0) (`GameplayStatics.GetPlayerController` 0))
          (`PlayerCameraManager.StartCameraFade` :`self` (`GameplayStatics.GetPlayerCameraManager` 0) :`ToAlpha` 1.0 :`Duration` (`self.FadeDuration`) :`bShouldFadeAudio` true)
          (`GameplayStatics.PlaySoundAtLocation` (`self.TransitionSound`) (`SceneComponent.K2_GetComponentLocation` (`self.StaticMesh`)) (struct) 1.0 1.0 0.0 null null null)
          (`KismetSystemLibrary.Delay` (`self.FadeDuration`))
          (`self.K2_TeleportTo` (`GameplayStatics.GetPlayerCharacter` 0) (`SceneComponent.K2_GetComponentLocation` _value) (`SceneComponent.K2_GetComponentRotation` _value))
          (set `self.CurrentCollider` null)
          (`PlayerCameraManager.StartCameraFade` :`self` (`GameplayStatics.GetPlayerCameraManager` 0) :`FromAlpha` 1.0 :`Duration` (`self.FadeDuration`) :`bShouldFadeAudio` true)
          (`KismetSystemLibrary.Delay` (`self.FadeDuration`))
          (`self.EnableInput` (`GameplayStatics.GetPlayerCharacter` 0) (`GameplayStatics.GetPlayerController` 0)))))))

(event `self.Front.OnComponentBeginOverlap`
  (params (OverlappedComponent :type "PrimitiveComponent Object Reference") (OtherActor :type "Actor Object Reference") (OtherComp :type "PrimitiveComponent Object Reference") (OtherBodyIndex :type Integer) (bFromSweep :type Boolean) (SweepResult :type "HitResult Structure (by ref)"))
  (set `self.CurrentCollider` (`self.Front`)))

(event `self.Front.OnComponentEndOverlap`
  (params (OverlappedComponent :type "PrimitiveComponent Object Reference") (OtherActor :type "Actor Object Reference") (OtherComp :type "PrimitiveComponent Object Reference") (OtherBodyIndex :type Integer))
  (set `self.CurrentCollider` null))

(event `self.Back.OnComponentBeginOverlap`
  (params (OverlappedComponent :type "PrimitiveComponent Object Reference") (OtherActor :type "Actor Object Reference") (OtherComp :type "PrimitiveComponent Object Reference") (OtherBodyIndex :type Integer) (bFromSweep :type Boolean) (SweepResult :type "HitResult Structure (by ref)"))
  (set `self.CurrentCollider` (`self.Back`)))

(event `self.Back.OnComponentEndOverlap`
  (params (OverlappedComponent :type "PrimitiveComponent Object Reference") (OtherActor :type "Actor Object Reference") (OtherComp :type "PrimitiveComponent Object Reference") (OtherBodyIndex :type Integer))
  (set `self.CurrentCollider` null))

(event `self.Unlock`
  (params (Key :type "/Game/Blueprints/Door/BP_Key Object Reference"))
  (if (== Key (`self.Key`))
    (set `self.IsLocked` false)
    (`GameplayStatics.PlaySoundAtLocation` "/Game/Sound/Door/door-unlock.door-unlock" (`self.K2_GetActorLocation`) (struct) 1.0 1.0 0.0 null null null)))

(event `self.Lock`
  (params (Key :type "/Game/Blueprints/Door/BP_Key Object Reference"))
  (if (== Key (`self.Key`))
    (set `self.IsLocked` true)))

(fn `UserConstructionScript`
  (`BlueprintMapLibrary.Map_Add` (`self.TeleportMapping`) (`self.Front`) (`self.TP_Position_Back`))
  (`BlueprintMapLibrary.Map_Add` (`self.TeleportMapping`) (`self.Back`) (`self.TP_Position_Front`)))