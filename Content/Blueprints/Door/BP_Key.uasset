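; BP_Key is a key pickup actor for a horror game, collected when the player character overlaps its box.
; On the first overlap only, it assigns itself to the character's Key variable, plays a pickup sound at its location and hides itself rather than being destroyed.
; It then prints a pickup message, fires a linked SpookTrigger and notifies the player through its notification component.
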(event `self.Box.OnComponentBeginOverlap`
  (params (OverlappedComponent :type "PrimitiveComponent Object Reference") (OtherActor :type "Actor Object Reference") (OtherComp :type "PrimitiveComponent Object Reference") (OtherBodyIndex :type Integer) (bFromSweep :type Boolean) (SweepResult :type "HitResult Structure (by ref)"))
  (bind _asdhbwhorror_character (cast `/Game/Blueprints/Character/DHBWHorrorCharacter` OtherActor))
  (`/Engine/EditorBlueprintResources/StandardMacros.DoOnce` false
    (:`Completed`
      (set `/Game/Blueprints/Character/DHBWHorrorCharacter.Key` self _asdhbwhorror_character)
      (`GameplayStatics.PlaySoundAtLocation` "/Game/Sound/Door/key-pick_up.key-pick_up" (`self.K2_GetActorLocation`) (struct) 1.0 1.0 0.0 null null null)
      (`self.SetActorHiddenInGame` true)
      (`KismetSystemLibrary.PrintString` "You picked up a key!")
      (`/Game/Blueprints/Spook/SpookTrigger.TriggerReceiver` (`self.SpookTrigger`))
      (`/Game/Blueprints/UI/NotificationComponent.NotifyPlayer` (`self.NotificationComponent`)))))

(fn `UserConstructionScript`)