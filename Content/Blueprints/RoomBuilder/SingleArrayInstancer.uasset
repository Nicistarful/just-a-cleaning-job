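; SingleArrayInstancer is a room-builder Blueprint that lays out a straight row of copies of one mesh.
; Its construction script applies the Mesh and Material variables to an InstancedStaticMesh component, then adds instances in a loop driven by Instances.
; Each instance is offset along Y by the mesh's bounds width, so copies sit edge to edge without manual spacing.
; The event graph is empty.
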(fn `UserConstructionScript`
  (bind (_returnvalue_origin _returnvalue_boxextent) (`KismetMathLibrary.BreakBoxSphereBounds` (`StaticMesh.GetBounds` (`StaticMeshComponent.StaticMesh` (`self.InstancedStaticMesh`)))))
  (`StaticMeshComponent.SetStaticMesh` (`self.InstancedStaticMesh`) (`self.Mesh`))
  (`PrimitiveComponent.SetMaterial` (`self.InstancedStaticMesh`) 0 (`self.Material`))
  (for _index (range (+ (`self.Instances`) 1))
    (`InstancedStaticMeshComponent.AddInstance` (`self.InstancedStaticMesh`) (`KismetMathLibrary.MakeTransform` (* (`KismetMathLibrary.MakeVector` 0.0 (* (.y _returnvalue_boxextent) 2.0)) _index)))))