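; Room builder Blueprint that procedurally assembles a rectangular room of floor, wall and ceiling mesh instances in its Construction Script.
; It loops over a Length by Width grid, spacing tiles by floor mesh bounds, raising flipped ceilings by wall height and placing rotated walls along the perimeter.
; Remover lists matched by tile location omit pieces, though removed floor tiles always get ceilings.
; Colored debug points mark each wall side.
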(fn `GetDebugPointPosition`
  (returns (ReturnValue :type "Vector Structure"))
  (return (`KismetMathLibrary.Conv_Vector2DToVector` (`self.GetMeshLocationAtIndex` (`self.FloorLoopIndex`)))))

(fn `GetFloorMeshSize`
  (returns (X :type "Float (double-precision)") (Y :type "Float (double-precision)"))
  (return (.x (* (`.BoxExtent` (`KismetMathLibrary.BreakBoxSphereBounds` (`StaticMesh.GetBounds` (`self.FloorStaticMesh`)))) 2.0)) (.y (* (`.BoxExtent` (`KismetMathLibrary.BreakBoxSphereBounds` (`StaticMesh.GetBounds` (`self.FloorStaticMesh`)))) 2.0))))

(fn `GetGridSize`
  (returns (ReturnValue :type Integer))
  (return (* (`self.Length`) (`self.Width`))))

(fn `GetMeshLocationAtIndex`
  (params (Index :type Integer))
  (returns (ReturnValue :type "Vector2D Structure"))
  (bind (_x _y) (`self.GetFloorMeshSize`))
  (return (`KismetMathLibrary.MakeVector2D` (* (mod Index (`self.Length`)) _x) (* (/ Index (`self.Length`)) _y))))

(fn `IsMeshAtIndexBorderPiece`
  (params (Index :type Integer))
  (returns (ReturnValue :type Boolean))
  (return (or (== (/ Index (`self.Length`)) 0) (== (mod (+ Index 1) (`self.Length`)) 0) (== (- (`self.Width`) 1) (/ Index (`self.Length`))) (== (mod Index (`self.Length`)) 0))))

(fn `IsMeshAtIndexCornerPiece`
  (params (Index :type Integer))
  (returns (ReturnValue :type Boolean))
  (return (or (== Index (- (`self.Length`) 1)) (== Index (- (* (`self.Width`) (`self.Length`)) 1)) (== Index (* (- (`self.Width`) 1) (`self.Length`))) (== Index 0))))

(fn `UserConstructionScript`
  (locals (BottomLeftCornerPosition :type "Vector2D Structure"))
  (bind _returnvalue (`KismetMathLibrary.Conv_Vector2DToVector` (`self.GetMeshLocationAtIndex` (`self.FloorLoopIndex`))))
  (`StaticMeshComponent.SetStaticMesh` (`self.FloorMesh`) (`self.FloorStaticMesh`))
  (`StaticMeshComponent.SetStaticMesh` (`self.WallMesh`) (`self.WallStaticMesh`))
  (`StaticMeshComponent.SetStaticMesh` (`self.CeilingMesh`) (`self.CeilingStaticMesh`))
  (`PrimitiveComponent.SetMaterial` (`self.FloorMesh`) 0 (`self.FloorMaterial`))
  (`PrimitiveComponent.SetMaterial` (`self.WallMesh`) 0 (`self.WallMaterial`))
  (`PrimitiveComponent.SetMaterial` (`self.CeilingMesh`) 0 (`self.CeilingMaterial`))
  (for _index (range (`self.GetGridSize`))
    (set `self.FloorLoopIndex` _index)
    (if (`KismetArrayLibrary.Array_Contains` (`self.FloorRemover`) (`KismetMathLibrary.Conv_Vector2DToVector` (`self.GetMeshLocationAtIndex` (`self.FloorLoopIndex`))))
      (`InstancedStaticMeshComponent.AddInstance` (`self.CeilingMesh`) (`KismetMathLibrary.MakeTransform` (+ _returnvalue (`KismetMathLibrary.MakeVector` 0.0 0.0 (* (.z (`.BoxExtent` (`KismetMathLibrary.BreakBoxSphereBounds` (`StaticMesh.GetBounds` (`self.WallStaticMesh`))))) 2.0))) (struct :`Roll` 180.0)) :!label _label)
      (else
        (`InstancedStaticMeshComponent.AddInstance` (`self.FloorMesh`) (`KismetMathLibrary.MakeTransform` _returnvalue))
        (if (`KismetArrayLibrary.Array_Contains` (`self.CeilingRemover`) (`KismetMathLibrary.Conv_Vector2DToVector` (`self.GetMeshLocationAtIndex` (`self.FloorLoopIndex`))))
          _
          (else
            (goto _label)))))
    (if (not (`KismetArrayLibrary.Array_Contains` (`self.WallRemover`) (`KismetMathLibrary.Conv_Vector2DToVector` (`self.GetMeshLocationAtIndex` (`self.FloorLoopIndex`)))))
      (`|ExecutionSequence`
        (:`then_0`
          (if (== (/ (`self.FloorLoopIndex`) (`self.Length`)) 0)
            (`KismetSystemLibrary.DrawDebugPoint` (`self.GetDebugPointPosition`) 32.0 (struct :`R` 1.0 :`A` 1.0) (`self.DebugPointDuration`))
            (`InstancedStaticMeshComponent.AddInstance` (`self.WallMesh`) (`KismetMathLibrary.MakeTransform` (- (`self.GetDebugPointPosition`) (`KismetMathLibrary.MakeVector` 0.0 (/ (`.Y` (`self.GetFloorMeshSize`)) 2.0))) (struct :`Yaw` 90.0)))))
        (:`then_1`
          (if (== (mod (+ (`self.FloorLoopIndex`) 1) (`self.Length`)) 0)
            (`KismetSystemLibrary.DrawDebugPoint` (`self.GetDebugPointPosition`) 32.0 (struct :`G` 1.0 :`A` 1.0) (`self.DebugPointDuration`))
            (`InstancedStaticMeshComponent.AddInstance` (`self.WallMesh`) (`KismetMathLibrary.MakeTransform` (+ (`self.GetDebugPointPosition`) (`KismetMathLibrary.MakeVector` (/ (`self.GetFloorMeshSize`) 2.0))) (struct :`Yaw` 180.0)))))
        (:`then_2`
          (if (== (- (`self.Width`) 1) (/ (`self.FloorLoopIndex`) (`self.Length`)))
            (`KismetSystemLibrary.DrawDebugPoint` (`self.GetDebugPointPosition`) 32.0 (struct :`B` 1.0 :`A` 1.0) (`self.DebugPointDuration`))
            (`InstancedStaticMeshComponent.AddInstance` (`self.WallMesh`) (`KismetMathLibrary.MakeTransform` (+ (`self.GetDebugPointPosition`) (`KismetMathLibrary.MakeVector` 0.0 (/ (`.Y` (`self.GetFloorMeshSize`)) 2.0))) (struct :`Yaw` -90.0)))))
        (:`then_3`
          (if (== (mod (`self.FloorLoopIndex`) (`self.Length`)) 0)
            (`KismetSystemLibrary.DrawDebugPoint` (`self.GetDebugPointPosition`) 32.0 (struct :`R` 1.0 :`G` 1.0 :`A` 1.0) (`self.DebugPointDuration`))
            (`InstancedStaticMeshComponent.AddInstance` (`self.WallMesh`) (`KismetMathLibrary.MakeTransform` (- (`self.GetDebugPointPosition`) (`KismetMathLibrary.MakeVector` (/ (`self.GetFloorMeshSize`) 2.0)))))))))))