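; Spook receiver lamp that flickers its light and plays a sound when triggered.
; BeginPlay assigns the configured sound to the audio component, and Trigger proceeds only if that sound is valid.
; A Flicker timeline drives the rect light's intensity, then swaps a mesh material slot to the off material when finished.
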(event `/Game/Blueprints/Spook/Triggerable.Trigger`
  (`/Engine/EditorBlueprintResources/StandardMacros.IsValid` (`AudioComponent.Sound` (`self.Audio`))
    (:`Is Valid`
      (`AudioComponent.Play` (`self.Audio`) 0.0)
      (bind (_direction _alpha) (`Timeline|Flicker`)
        (:`Update`
          (`LightComponent.SetIntensity` (`self.RectLight`) (`KismetMathLibrary.Lerp` 0.0 8.0 _alpha)))
        (:`Finished`
          (`PrimitiveComponent.SetMaterial` (`self.StaticMesh`) 1 (`self.MaterialOff`)))))))

(event `self.ReceiveBeginPlay`
  (`AudioComponent.SetSound` (`self.Audio`) (`self.Sound`)))

(fn `UserConstructionScript`
  (`parent.UserConstructionScript`))