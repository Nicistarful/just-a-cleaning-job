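; SpookTrigger is a Blueprint that fires a scare by sending TriggerMessage to its SpookTarget.
; On BeginPlay, if UseTrigger is set, it binds an overlap handler to its Trigger actor's begin-overlap event.
; Overlaps, or direct TriggerReceiver calls, forward the message only while PlaySpook is true, with no check on which actor overlapped.
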(event `TriggerReceiver`
  (if (`self.PlaySpook`)
    (message `/Game/Blueprints/Spook/Triggerable.Trigger` (`self.SpookTarget`))))

(event `self.ReceiveBeginPlay`
  (if (`self.UseTrigger`)
    (add `Actor.OnActorBeginOverlap` (`self.Trigger`) (delegate `OnPlayerOverlap`))))

(event `OnPlayerOverlap`
  (params (OverlappedActor :type "Actor Object Reference") (OtherActor :type "Actor Object Reference"))
  (`self.TriggerReceiver`))