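; Sprint component for DHBWHorrorCharacter that gradually ramps the character's walk speed up while sprinting and back down afterwards.
; StartSprint and StopSprint toggle a flag that a looping timer reads to accelerate or decelerate, clamped between the default walk speed and the sprint maximum.
; The result is written to CharacterMovement's MaxWalkSpeed.
; Tick prints current speed and planar velocity as debug text, and EndPlay clears the timer.
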(event `self.ReceiveBeginPlay`
  (bind _asdhbwhorror_character (cast `/Game/Blueprints/Character/DHBWHorrorCharacter` (`self.GetOwner`)))
  (bind _output_get (set `self.As DHBWHorror Character` _asdhbwhorror_character))
  (bind _output_get_2 (set `self.Character Movement` (`Character.CharacterMovement` _output_get)))
  (set `self.DefaultMaxWalkSpeed` (`CharacterMovementComponent.MaxWalkSpeed` _output_get_2))
  (bind _returnvalue (`KismetSystemLibrary.K2_SetTimerDelegate` (`|CreateDelegate` :!event `SprintTimerUpdate`) (`self.Interval`) true))
  (set `self.SprintTimerHandle` _returnvalue))

(event `Start Sprint`
  (set `self.Sprinting` true))

(event `SprintTimerUpdate`
  (bind _output_get (set `self.CurrentSpeed` (`KismetMathLibrary.FClamp` (select `bool` (`self.Sprinting`) :`false` (- (`self.CurrentSpeed`) (`self.Deacceleration`)) :`true` (+ (`self.CurrentSpeed`) (`self.Acceleration`))) (`self.DefaultMaxWalkSpeed`) (`self.MaxSprintSpeed`))))
  (set `CharacterMovementComponent.MaxWalkSpeed` _output_get (`self.Character Movement`)))

(event `Stop Sprint`
  (set `self.Sprinting` false))

(event `self.ReceiveEndPlay`
  (params (EndPlayReason :type "EEndPlayReason Enum" :default "Destroyed"))
  (`KismetSystemLibrary.K2_ClearAndInvalidateTimerHandle` (`self.SprintTimerHandle`)))

(event `self.ReceiveTick`
  (params (DeltaSeconds :type "Float (single-precision)"))
  (`KismetSystemLibrary.PrintText` (`|FormatText` "Current Speed: {CurrentSpeed} \nVelocity: {Velocity} u/s" (`self.CurrentSpeed`) (`/Game/Blueprints/Character/DHBWHorrorCharacter.GetPlanarVelocity` (`self.As DHBWHorror Character`))) true false (struct :`G` 0.66 :`B` 1.0 :`A` 1.0) 0.0))