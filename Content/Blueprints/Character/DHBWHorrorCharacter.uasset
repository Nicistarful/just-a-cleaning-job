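; First-person player character for a horror game, handling movement, look, sprint and interaction input.
; Interact line-traces a short distance from the camera and sends InteractMessage with Key to the hit actor; sprint is delegated to SprintComponent.
; Movement input is scaled by floor slope, with calls signalling walk start/stop and leaving or reaching ground.
; FootstepComponent steps trigger left/right headbob camera anims, scaled by planar speed against max sprint speed.
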(event `InputAction|Interact`
  (params (Key :type "Key Structure"))
  (bind _camera (`self.Camera`))
  (bind _returnvalue (`SceneComponent.K2_GetComponentLocation` _camera))
  (:`Pressed`
    (bind _outhit (`KismetSystemLibrary.LineTraceSingle` :`Start` _returnvalue :`End` (+ _returnvalue (* (`KismetMathLibrary.GetForwardVector` (`SceneComponent.K2_GetComponentRotation` _camera)) 100.0)) :`TraceChannel` "TraceTypeQuery1" :`DrawDebugType` "ForDuration"))
    (message `/Game/Blueprints/Interfaces/Interaction.Interact` (`.HitActor` (`GameplayStatics.BreakHitResult` _outhit)) (`self.Key`))))

(event `InputAction|Sprint`
  (params (Key :type "Key Structure"))
  (bind _sprintcomponent (`self.SprintComponent`))
  (:`Pressed`
    (`/Game/Blueprints/Character/SprintComponent.Start Sprint` _sprintcomponent))
  (:`Released`
    (`/Game/Blueprints/Character/SprintComponent.Stop Sprint` _sprintcomponent)))

(event `InputAxis|MoveForward`
  (params (AxisValue :type "Float (single-precision)"))
  (`self.AddMovementInput` (* (`self.GetAbsoluteFloorNormal` (`self.SlopeIntensity`)) (`self.GetActorForwardVector` (`GameplayStatics.GetPlayerPawn` 0))) AxisValue)
  (if (and (== AxisValue 0.0) (== (stale `InputAxis|MoveRight` AxisValue) 0.0)) :!label _label
    (`/Engine/EditorBlueprintResources/StandardMacros.DoOnce` true :!label _label_2
      (:`Completed`
        (`self.OnStoppedWalking`)
        (goto _label_3 :!via `Reset`)))
    (else
      (`/Engine/EditorBlueprintResources/StandardMacros.DoOnce` false :!label _label_3
        (:`Completed`
          (`self.OnStartedWalking`)
          (goto _label_2 :!via `Reset`))))))

(event `InputAxis|MoveRight`
  (params (AxisValue :type "Float (single-precision)"))
  (`self.AddMovementInput` (* (`self.GetAbsoluteFloorNormal` (`self.SlopeIntensity`)) (`self.GetActorRightVector` (`GameplayStatics.GetPlayerPawn` 0))) AxisValue)
  (goto _label))

(event `InputAxis|LookRight`
  (params (AxisValue :type "Float (single-precision)"))
  (`self.AddControllerYawInput` AxisValue))

(event `InputAxis|LookUp`
  (params (AxisValue :type "Float (single-precision)"))
  (`self.AddControllerPitchInput` AxisValue))

(event `self.OnLanded`
  (params (Hit :type "HitResult Structure (by ref)"))
  (`self.OnReachedGround`))

(event `self.OnWalkingOffLedge`
  (params (PreviousFloorImpactNormal :type "Vector Structure (by ref)") (PreviousFloorContactNormal :type "Vector Structure (by ref)") (PreviousLocation :type "Vector Structure (by ref)") (TimeDelta :type "Float (single-precision)"))
  (`self.OnLeftGround` :!label _label_4))

(event `self.OnLaunched`
  (params (LaunchVelocity :type "Vector Structure") (bXYOverride :type Boolean) (bZOverride :type Boolean))
  (goto _label_4))

(event `self.OnJumped`
  (goto _label_4))

(event `self.FootstepComponent.OnFootstep`
  (bind _returnvalue (/ (`self.GetPlanarVelocity`) (`/Game/Blueprints/Character/SprintComponent.MaxSprintSpeed` (`self.SprintComponent`))))
  (`PlayerCameraManager.PlayCameraAnim` :`self` (`GameplayStatics.GetPlayerCameraManager` 0) :`Anim` (select `bool` (`/Game/Blueprints/Character/FootstepComponent.IsRightFoot` (`self.FootstepComponent`)) :`false` "/Game/Blueprints/Character/LeftHeadbobCameraAnim.LeftHeadbobCameraAnim" :`true` "/Game/Blueprints/Character/RightHeadbobCameraAnim.RightHeadbobCameraAnim" :!type "CameraAnim Object Reference") :`Rate` (`KismetMathLibrary.Lerp` (`self.MinHeadbobRate`) (`self.MaxHeadbobRate`) _returnvalue) :`Scale` (`KismetMathLibrary.Lerp` 0.0 1.0 _returnvalue)))

(fn `GetAbsoluteFloorNormal`
  (params (Intensity :type "Float (double-precision)" :default 1.0))
  (returns (ReturnValue :type "Vector Structure"))
  (return (* (`KismetMathLibrary.MakeVector` (- 1.0 (`KismetMathLibrary.Abs` (.x (`.Normal` (`GameplayStatics.BreakHitResult` (`.HitResult` (break `FindFloorResult` (`CharacterMovementComponent.CurrentFloor` (`self.CharacterMovement`))))))))) (- 1.0 (`KismetMathLibrary.Abs` (.y (`.Normal` (`GameplayStatics.BreakHitResult` (`.HitResult` (break `FindFloorResult` (`CharacterMovementComponent.CurrentFloor` (`self.CharacterMovement`)))))))))) Intensity)))

(fn `GetPlanarVelocity`
  (returns (ReturnValue :type "Float (double-precision)"))
  (return (`KismetMathLibrary.VSize` (`KismetMathLibrary.MakeVector` (.x (`MovementComponent.Velocity` (`self.CharacterMovement`))) (.y (`MovementComponent.Velocity` (`self.CharacterMovement`)))))))

(fn `UserConstructionScript`)