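; Footstep component for DHBWHorrorCharacter that plays surface-dependent step sounds while the character walks on the ground.
; Walk and ground events from the character start or cancel a self-requeuing timer whose interval shrinks as planar velocity rises.
; Each step traces down for the surface type, picks a sound from a map with a concrete fallback, alternates pitch per foot and fires a footstep event.
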(event `self.ReceiveBeginPlay`
  (bind _asdhbwhorror_character (cast `/Game/Blueprints/Character/DHBWHorrorCharacter` (`self.GetOwner`)))
  (bind _output_get (set `self.DHBWHorrorCharacter` _asdhbwhorror_character))
  (set `self.Character Movement` (`Character.CharacterMovement` _output_get))
  (add `/Game/Blueprints/Character/DHBWHorrorCharacter.OnStartedWalking` (`self.DHBWHorrorCharacter`) (`|CreateDelegate` :!event `OnStartedWalking`))
  (add `/Game/Blueprints/Character/DHBWHorrorCharacter.OnStoppedWalking` (`self.DHBWHorrorCharacter`) (`|CreateDelegate` :!event `OnStoppedWalking`))
  (add `/Game/Blueprints/Character/DHBWHorrorCharacter.OnLeftGround` (`self.DHBWHorrorCharacter`) (`|CreateDelegate` :!event `OnLeftGround`))
  (add `/Game/Blueprints/Character/DHBWHorrorCharacter.OnReachedGround` (`self.DHBWHorrorCharacter`) (`|CreateDelegate` :!event `OnReachedGround`)))

(event `OnStartedWalking`
  (`KismetSystemLibrary.PrintString` "Started Walking" :!label _label)
  (set `self.IsMoving` true)
  (`self.QueueFootstep` 0.1))

(event `OnReachedGround`
  (goto _label))

(event `OnStoppedWalking`
  (`KismetSystemLibrary.PrintString` "Stopped Walking")
  (set `self.IsMoving` false :!label _label_2)
  (`KismetSystemLibrary.K2_ClearAndInvalidateTimerHandle` (`self.QueuedFootstepHandle`)))

(event `OnLeftGround`
  (`KismetSystemLibrary.PrintString` "Left Ground")
  (goto _label_2))

(event `Footstep`
  (bind _counter (`self.Counter`))
  (bind _result (`/Engine/EditorBlueprintResources/StandardMacros.IncrementInt` _counter)
    (:`  `
      (`KismetSystemLibrary.PrintString` (`KismetStringLibrary.Conv_IntToString` _result))
      (set `self.IsRightFoot` (== (mod _counter 2) 0))
      (bind (_hitresult _returnvalue) (`self.GetFloorHitResult`))
      (if _returnvalue
        (`GameplayStatics.SpawnSoundAtLocation` (`self.GetStepSound` (`GameplayStatics.GetSurfaceType` _hitresult)) (`.Location` (`GameplayStatics.BreakHitResult` _hitresult)) (struct) 1.0 (select `bool` (`self.IsRightFoot`) :`false` 1.0 :`true` 1.05 :!type "Float (single-precision)") 0.0 null null)
        (`self.OnFootstep`)
        (if (`self.IsMoving`)
          (`self.QueueFootstep` (`self.GetStepFrequency`)))))))

(event `QueueFootstep`
  (params (Time :type "Float (double-precision)"))
  (bind _returnvalue (`KismetSystemLibrary.K2_SetTimerDelegate` (`|CreateDelegate` :!event `Footstep`) Time))
  (set `self.QueuedFootstepHandle` _returnvalue))

(fn `GetFloorHitResult`
  (returns (HitResult :type "HitResult Structure") (ReturnValue :type Boolean))
  (bind _returnvalue (`self.GetOwner`))
  (bind _returnvalue_2 (`Actor.K2_GetActorLocation` _returnvalue))
  (bind (_outhit _returnvalue_3) (`KismetSystemLibrary.LineTraceSingle` _returnvalue_2 (- _returnvalue_2 (0.0 0.0 200.0)) "TraceTypeQuery1" false (`|MakeArray` _returnvalue)))
  (return _outhit _returnvalue_3))

(fn `GetStepFrequency`
  (returns (ReturnValue :type "Float (double-precision)"))
  (return (/ 1.0 (* (`/Game/Blueprints/Character/DHBWHorrorCharacter.GetPlanarVelocity` (`self.DHBWHorrorCharacter`)) 0.0075))))

(fn `GetStepSound`
  (params (Key :type "EPhysicalSurface Enum (by ref)"))
  (returns (Value :type "SoundCue Object Reference"))
  (bind (_value _returnvalue) (`BlueprintMapLibrary.Map_Find` (`self.Sounds`) Key))
  (if _returnvalue
    (return _value)
    (else
      (return "/Game/Sound/Steps/ConcreteCue.ConcreteCue"))))